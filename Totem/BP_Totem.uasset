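; Interactable totem of green, pink or blue type that spawns a matching key and reports its activation to BP_GameMode.
; On Interact, each type branch runs once, spawning the key at an arrow, incrementing the active-totem count and checking all totems.
; Only the visual activation depends on the GameMode's picked-key flag: it plays the square's movement timeline and brightens a dynamic glow material created in the construction script.
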(event Custom|ActiveTotemGreen
  ;[1 1 1] Pick Key / Play Animation
  (if (Variables|/Game/HeroCharacter/GameLoop/BP_GameMode.BP_GameMode_C|GetIsPickKeyGreen (Variables|Default|GetGame%20Mode%20Refer))
    (Components|Timeline|PlayfromStart (Variables|Default|GetSquard%20Timeline))
    (Rendering|Material|SetScalarParameterValue (Variables|Default|GetTotem%20Mat) "Emissive" (Variables|Default|GetEmissiveActiveIntensity) :!class /Script/Engine.MaterialInstanceDynamic)))

(event Custom|ActiveTotemPinkKey
  ;[1 1 1] Pick Key / Play Animation
  (if (Variables|/Game/HeroCharacter/GameLoop/BP_GameMode.BP_GameMode_C|GetIsPickKeyPink (Variables|Default|GetGame%20Mode%20Refer))
    (Components|Timeline|PlayfromStart (Variables|Default|GetSquard%20Timeline))
    (Rendering|Material|SetScalarParameterValue (Variables|Default|GetTotem%20Mat) "Emissive" (Variables|Default|GetEmissiveActiveIntensity) :!class /Script/Engine.MaterialInstanceDynamic)))

(event Custom|ActiveTotemBlueKey
  ;[1 1 1] Pick Key / Play Animation
  (if (Variables|/Game/HeroCharacter/GameLoop/BP_GameMode.BP_GameMode_C|GetIsPickKeyBlue (Variables|Default|GetGame%20Mode%20Refer))
    (Components|Timeline|PlayfromStart (Variables|Default|GetSquard%20Timeline))
    (Rendering|Material|SetScalarParameterValue (Variables|Default|GetTotem%20Mat) "Emissive" (Variables|Default|GetEmissiveActiveIntensity) :!class /Script/Engine.MaterialInstanceDynamic)))

(event Collision|EventActorBeginOverlap
  (params (OtherActor :type Actor%20Object%20Reference)))

(event EventTick
  (params (DeltaSeconds :type Float%20%28single-precision%29)))

(event EventInteract
  (bind _game_mode_refer (Variables|Default|GetGame%20Mode%20Refer))
  (bind _game_mode_refer_2 (Variables|Default|GetGame%20Mode%20Refer))
  (bind _game_mode_refer_3 (Variables|Default|GetGame%20Mode%20Refer))
  ;[1 1 1] Blueprint Interface Interact --Active Totem Spawn Key
  (switch Utilities|FlowControl|Switch|SwitchonEKey (Variables|Default|GetTotemType)
    (:NewEnumerator0
      (Utilities|FlowControl|DoOnce false
        (:Completed
          (CallFunction|ActiveTotemGreen)
          (CallFunction|SpawnKeyGreen)
          (Default|IncreamentNumberTotamActive _game_mode_refer)
          (Default|CheckAllActiveTotam _game_mode_refer))))
    (:NewEnumerator1
      (Utilities|FlowControl|DoOnce false
        (:Completed
          (CallFunction|ActiveTotemPinkKey)
          (CallFunction|SpawnPinkKey)
          (Default|IncreamentNumberTotamActive _game_mode_refer_2)
          (Default|CheckAllActiveTotam _game_mode_refer_2))))
    (:NewEnumerator2
      (Utilities|FlowControl|DoOnce false
        (:Completed
          (CallFunction|ActiveTotemBlueKey)
          (CallFunction|SpawnBlueKey)
          (Default|IncreamentNumberTotamActive _game_mode_refer_3)
          (Default|CheckAllActiveTotam _game_mode_refer_3))))))

(event EventBeginPlay
  (bind _asbp_game_mode (Utilities|Casting|CastToBP_GameMode (Game|GetGameMode)))
  (Variables|Default|SetGame%20Mode%20Refer _asbp_game_mode))

(fn ConstructionScript
  (bind _returnvalue (Rendering|Material|CreateDynamicMaterialInstance (Variables|Default|GetTotamBase) 1 "/Game/HeroCharacter/Materials/M_Glow.M_Glow" "None" :!class /Script/Engine.PrimitiveComponent))
  (bind _output_get (Variables|Default|SetTotem%20Mat _returnvalue))
  (Rendering|Material|SetScalarParameterValue _output_get "Emissive" (Variables|Default|GetEmissive%20Intensity) :!class /Script/Engine.MaterialInstanceDynamic)
  (Rendering|Material|SetVectorParameterValue _output_get "BaseColor" (Variables|Default|GetBaseColor) :!class /Script/Engine.MaterialInstanceDynamic))

(fn SpawnKeyGreen
  (Game|SpawnActorfromClass "/Game/HeroCharacter/Object/Key/BP_KeyFixed2.BP_KeyFixed2_C" (Transformation|GetWorldTransform (Variables|Default|GetArrowTransform)) "Undefined" 0 0)
  (return 0))

(fn SpawnBlueKey
  (Game|SpawnActorfromClass "/Game/HeroCharacter/Object/Key/BP_KeyFixed.BP_KeyFixed_C" (Transformation|GetWorldTransform (Variables|Default|GetArrowTransform)) "Undefined" 0 0)
  (return 0))

(fn SpawnPinkKey
  (Game|SpawnActorfromClass "/Game/HeroCharacter/Object/Key/BP_KeyFixed1.BP_KeyFixed1_C" (Transformation|GetWorldTransform (Variables|Default|GetArrowTransform)) "Undefined" 0 0)
  (return 0))