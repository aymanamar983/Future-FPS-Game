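; Enemy Blueprint for a bobbing shooter that turns to face the player and fires projectiles once the player is detected.
; A capsule overlap or a hit sets detection flags, and Tick then starts a looping Fire timer through a resettable DoOnce.
; The EnemyLoop timeline lerps between randomized vertical endpoints at a random rate.
; Hits reduce health and flash the emissive material, or trigger death and destroy the actor at zero.
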(event OnComponentBeginOverlap(Capsule)
  (params (OverlappedComponent :type Primitive%20Component%20Object%20Reference) (OtherActor :type Actor%20Object%20Reference) (OtherComp :type Primitive%20Component%20Object%20Reference) (OtherBodyIndex :type Integer) (bFromSweep :type Boolean) (SweepResult :type Hit%20Result%20Structure%20%28by%20ref%29))
  ;[1 1 1] Set Palyer - Overlap
  (Variables|Default|SetIsPlayeronSight true))

(event Custom|StopEnemy
  ;[1 1 1] Stop Enemy
  (Utilities|Time|ClearTimerbyFunctionName 0 "Fire"))

(event Custom|RestartEnemyFire
  ;[1 1 1] Enemy See Player Fire
  (Utilities|FlowControl|DoOnce false) ; enters at Reset
)

(event Custom|RestartEnemy
  ;[1 1 1] ResetEnemy
  (Variables|Default|SetIsPlayeronSight false)
  (Variables|Default|SetIsPlayerHere false))

(event Custom|Event%20Dead)

(event EventBeginPlay
  (bind _returnvalue (Transformation|GetActorLocation))
  (Utilities|FlowControl|Sequence
    (:then_0
      ;[1 1 1] Set Start / End Location - Timeline Loop
      (Variables|Default|SetStart%20Location _returnvalue)
      (Variables|Default|SetEnd%20Location (+ _returnvalue (Math|Vector|MakeVector 0.0 0.0 (Math|Random|RandomFloatinRange 5e+01 1e+02))))
      (Components|Timeline|SetPlayRate (Variables|Default|GetEnemyLoop) (Math|Random|RandomFloatinRange 1.0 2.0)))
    (:then_1
      ;[1 1 1] Player Refer
      (bind _asbp_player (Utilities|Casting|CastToBP_Player (Game|GetPlayerCharacter 0)))
      (Variables|Default|Set%20Player%20refer _asbp_player))))

(event Collision|EventHit
  (params (MyComp :type Primitive%20Component%20Object%20Reference) (Other :type Actor%20Object%20Reference) (OtherComp :type Primitive%20Component%20Object%20Reference) (bSelfMoved :type Boolean) (HitLocation :type Vector :default "0, 0, 0") (HitNormal :type Vector :default "0, 0, 0") (NormalImpulse :type Vector :default "0, 0, 0") (Hit :type Hit%20Result%20Structure%20%28by%20ref%29))
  ;[1 1 1] Enemy Health and Damage
  (Audio|PlaySoundatLocation "/Game/HeroCharacter/Audio/grenade2_Cue.grenade2_Cue" HitLocation "0, 0, 0" 1.0 1.0 0.0 0 0 0)
  (Variables|Default|SetIsPlayerHere true)
  (Variables|Default|SetEnemyHealth (- (Variables|Default|GetEnemyHealth) (Variables|Default|GetDamageTaken)))
  (if (<= (Variables|Default|GetEnemyHealth) 0.0)
    (CallFunction|EventDead)
    (Actor|DestroyActor)
    (else
      (Rendering|Material|SetScalarParameterValueonMaterials (Variables|Default|GetEnemyMesh) "Emissive" 1.0)
      (Utilities|FlowControl|Delay 0.1)
      (Rendering|Material|SetScalarParameterValueonMaterials (Variables|Default|GetEnemyMesh) "Emissive" 6e+01))))

(event EventTick
  (params (DeltaSeconds :type Float%20%28single-precision%29))
  ;[1 1 1] Enemy See Player Fire
  (if (or (Variables|Default|GetIsPlayeronSight) (Variables|Default|GetIsPlayerHere))
    (Utilities|FlowControl|Sequence
      (:then_0
        (Transformation|SetActorRotation (Math|Rotator|FindLookatRotation (Transformation|GetActorLocation) (Transformation|GetActorLocation (Variables|Default|Get%20Player%20refer)))))
      (:then_1
        (Utilities|FlowControl|DoOnce false
          (:Completed
            (Utilities|Time|SetTimerbyFunctionName 0 "Fire" (/ 1.0 (Variables|Default|GetShootPerSeconds)) true)))))))

(fn ConstructionScript)

(fn Fire
  (bind _arrowprojectile (Variables|Default|GetArrowProjectile))
  (Game|SpawnActorfromClass "/Game/HeroCharacter/Enemy/BP_EnemyProjectile.BP_EnemyProjectile_C" (Transformation|GetWorldTransform _arrowprojectile) "Undefined" 0 0)
  (Audio|PlaySoundatLocation "/Game/HeroCharacter/Audio/tiro6_Cue.tiro6_Cue" (Transformation|GetWorldLocation _arrowprojectile) "0, 0, 0" 1.0 1.0 0.0 0 0 0))