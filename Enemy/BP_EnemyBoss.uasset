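; BP_EnemyBoss is a boss enemy that counts toward the game's win condition when it dies.
; On BeginPlay it runs the parent logic, then caches a cast reference to BP_GameMode.
; When the parent class calls EventDead, it increments the game mode's count of dead bosses and calls CheckWin.
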(event EventBeginPlay
  (|CallParentFunction)
  ;[1 1 1] GameModeRefer
  (bind _asbp_game_mode (Utilities|Casting|CastToBP_GameMode (Game|GetGameMode)))
  (Variables|Default|SetGame%20Mode%20Refer _asbp_game_mode))

(event Collision|EventActorBeginOverlap
  (params (OtherActor :type Actor%20Object%20Reference)))

(event EventTick
  (params (DeltaSeconds :type Float%20%28single-precision%29))
  (|CallParentFunction DeltaSeconds) ; This node is disabled and will not be called.\nDrag off pins to build functionality.
)

(event EventEventDead
  (bind _game_mode_refer (Variables|Default|GetGame%20Mode%20Refer))
  ;[1 1 1] When Parents Class Calls EventDead , we increased number of Bosses Dead And Check WinGame
  (Variables|/Game/HeroCharacter/GameLoop/BP_GameMode.BP_GameMode_C|SetNumber%20Of%20Enemy%20Bosses%20Dead _game_mode_refer (+ (Variables|/Game/HeroCharacter/GameLoop/BP_GameMode.BP_GameMode_C|GetNumber%20Of%20Enemy%20Bosses%20Dead _game_mode_refer) 1))
  (Default|CheckWin (Variables|Default|GetGame%20Mode%20Refer)))

(fn ConstructionScript
  (|CallParentFunction))