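; SKGun_BP is an automatic gun that fires BP_Projectile from the player character.
; On BeginPlay it caches the BP_Player reference.
; ActiveTrigger fires immediately, then repeats Fire on a looping timer set by ShootPerSeconds until DeactiveTrigger clears it.
; Each shot spawns the projectile and a shot sound at the player's Arrow1 component rather than at a muzzle on the gun.
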(event Custom|ActiveTrigger
  ;[1 1 1] Active/Deactive - Trigger
  (CallFunction|Fire)
  (Utilities|Time|SetTimerbyFunctionName 0 "Fire" (/ 1.0 (Variables|Default|GetShootPerSeconds)) true))

(event Custom|DeactiveTrigger
  ;[1 1 1] Active/Deactive - Trigger
  (Utilities|Time|ClearTimerbyFunctionName 0 "Fire"))

(event EventBeginPlay
  ;[1 1 1] Get Player Refer
  (bind _asbp_player (Utilities|Casting|CastToBP_Player (Game|GetPlayerCharacter 0)))
  (Variables|Default|SetPlayer%20Refer _asbp_player))

(fn ConstructionScript)

(fn Fire
  (bind _player_refer (Variables|Default|GetPlayer%20Refer))
  (bind _arrow1 (Variables|/Game/HeroCharacter/BP_Player.BP_Player_C|GetArrow1 _player_refer))
  (bind _returnvalue (Transformation|GetWorldTransform _arrow1))
  (Game|SpawnActorfromClass "/Game/HeroCharacter/BP_Projectile.BP_Projectile_C" (Math|Transform|MakeTransform (.location _returnvalue) (.rotation _returnvalue) (.scale _returnvalue)) "Undefined" 0 0)
  (Audio|SpawnSoundatLocation "/Game/HeroCharacter/Audio/tiro4_Cue.tiro4_Cue" (.location _returnvalue) "0, 0, 0" 1.0 1.0 0.0 0 0))