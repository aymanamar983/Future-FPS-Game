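; Game mode that runs the level loop: player HUD, pause and death menus, key pickups, win conditions and checkpoint respawn.
; BeginPlay creates the widgets, plays music, binds player events and counts totems, plus bosses in BossLevel.
; Activating all totems or killing all bosses spawns a level portal.
; On death, the controller possesses the first checkpoint found and enemies stop; restarting repossesses the player there, resets health and restarts enemies.
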(event Custom|PlayerDead
  ;[1 1 1] PlayerIsDead
  (CallFunction|HideHeroCharacter)
  (CallFunction|PossessCheckPoint)
  (CallFunction|StopAllEnemies)
  (CallFunction|AddDeadMenuHidePlayerHUD)
  (EventDispatchers|AssignRestartfromCheckpoint (Variables|Default|GetMenu%20Dead) (delegate Custom|RestartFromCheckpoint)))

(event Custom|UpdateUI
  (bind _player_refer (Variables|Default|GetPlayer%20Refer))
  (bind _currenthealth (Variables|/Game/HeroCharacter/BP_Player.BP_Player_C|GetCurrentHealth _player_refer))
  ;[1 1 1] UpdateUI
  (Variables|/Game/HeroCharacter/HUD/HUD_Player.HUD_Player_C|SetHealthHUD (Variables|Default|GetHUDPlayerRefer) (Utilities|Text|ToText(Float) _currenthealth "HalfToEven"))
  (if (<= _currenthealth 0.0)
    (Variables|/Game/HeroCharacter/HUD/HUD_Player.HUD_Player_C|SetProgress%20HUD (Variables|Default|GetHUDPlayerRefer) 0.0)
    (else
      (Variables|/Game/HeroCharacter/HUD/HUD_Player.HUD_Player_C|SetProgress%20HUD (Variables|Default|GetHUDPlayerRefer) (/ _currenthealth 1e+02)))))

(event Custom|pauseGame
  (bind _returnvalue (Game|GetPlayerController 0))
  (bind _menupauserefer (Variables|Default|GetMenuPauseRefer))
  ;[1 1 1] Pause/Unpause MENU
  (Game|SetGamePaused true)
  (Widget|RemovefromParent (Variables|Default|GetHUDPlayerRefer))
  (UserInterface|Viewport|AddtoViewport _menupauserefer 0)
  (Variables|/Script/Engine.PlayerController|SetbShowMouseCursor _returnvalue true)
  (Input|SetInputModeUIOnly _returnvalue _menupauserefer "DoNotLock"))

(event Custom|UnpauseGame
  (bind _returnvalue (Game|GetPlayerController 0))
  ;[1 1 1] Pause/Unpause MENU
  (Game|SetGamePaused false)
  (Widget|RemovefromParent (Variables|Default|GetMenuPauseRefer))
  (UserInterface|Viewport|AddtoViewport (Variables|Default|GetHUDPlayerRefer) 0)
  (Variables|/Script/Engine.PlayerController|SetbShowMouseCursor _returnvalue false)
  (Input|SetInputModeGameOnly _returnvalue))

(event Custom|RestartFromCheckpoint
  ;[1 1 1] Restart Game Function
  (Utilities|FlowControl|Sequence
    (:then_0
      (CallFunction|PossesPlayer)
      (CallFunction|UnHideHeroCharacter0)
      (CallFunction|SetPlayerPosition)
      (CallFunction|RestartPlayer))
    (:then_1
      (CallFunction|RemoveDeadMenuHidePlayerHUD0)
      (CallFunction|UpdateUI))
    (:then_2
      (CallFunction|RestartAllEnemies))))

(event Custom|PickBlueKey_Event
  ;[1 1 1] AssignKeysPickup
  (CallFunction|IncreamentNumberKeys)
  (Default|ChanceKeyBlue (Variables|Default|GetHUDPlayerRefer))
  (Variables|Default|SetIsPickKeyBlue true))

(event Custom|PickGreenKey_Event
  ;[1 1 1] AssignKeysPickup
  (CallFunction|IncreamentNumberKeys)
  (Default|ChangeKeyGreen (Variables|Default|GetHUDPlayerRefer))
  (Variables|Default|SetIsPickKeyGreen true))

(event Custom|PickPinkKey_Event
  ;[1 1 1] AssignKeysPickup
  (CallFunction|IncreamentNumberKeys)
  (Default|ChangeKeyPink (Variables|Default|GetHUDPlayerRefer))
  (Variables|Default|SetIsPickKeyPink true))

(event Custom|AllActiveTotam_Event_0
  ;[1 1 1] GetTotamNumber -- Assign ActiveTotam
  (Game|SpawnActorfromClass "/Game/HeroCharacter/Portal/BP_PortalFrame.BP_PortalFrame_C" (Variables|Default|GetPortalLevelSpawnTransform) "Undefined" 0 "BossLevel" 0))

(event EventBeginPlay
  (Utilities|FlowControl|Sequence
    (:then_0
      ;[1 1 1] Player Refer
      (bind _asbp_player (Utilities|Casting|CastToBP_Player (Game|GetPlayerCharacter 0)))
      (Variables|Default|SetPlayer%20Refer _asbp_player)
      (Audio|PlaySound2D "/Game/HeroCharacter/Audio/The_Grid_-_Electrified__Gameplay__Cue.The_Grid_-_Electrified__Gameplay__Cue" 1.0 1.0 0.0 0 0))
    (:then_1
      ;[1 1 1] HUD player
      (bind _returnvalue (UserInterface|CreateWidget "/Game/HeroCharacter/HUD/HUD_Player.HUD_Player_C" (Game|GetPlayerController 0)))
      (bind _output_get (Variables|Default|SetHUDPlayerRefer _returnvalue))
      (UserInterface|Viewport|AddtoViewport _output_get 0))
    (:then_2
      ;[1 1 1] MenuPauseHUD
      (bind _returnvalue_2 (UserInterface|CreateWidget "/Game/HeroCharacter/HUD/MenuPause.MenuPause_C" (Game|GetPlayerController 0)))
      (Variables|Default|SetMenuPauseRefer _returnvalue_2))
    (:then_3
      ;[1 1 1] MenuDeadHUD
      (bind _returnvalue_3 (UserInterface|CreateWidget "/Game/HeroCharacter/HUD/MenuDead.MenuDead_C" (Game|GetPlayerController 0)))
      (Variables|Default|SetMenu%20Dead _returnvalue_3))
    (:then_4
      ;[1 1 1] AssignKeysPickup
      (EventDispatchers|AssignPickBlueKey (Variables|Default|GetPlayer%20Refer) (delegate Custom|PickBlueKey_Event))
      (EventDispatchers|AssignPickGreenKey (Variables|Default|GetPlayer%20Refer) (delegate Custom|PickGreenKey_Event))
      (EventDispatchers|AssignPickPinkKey (Variables|Default|GetPlayer%20Refer) (delegate Custom|PickPinkKey_Event)))
    (:then_5
      ;[1 1 1] GetTotamNumber -- Assign ActiveTotam
      (bind _outactors (Actor|GetAllActorsOfClass "/Game/HeroCharacter/Totem/BP_Totem.BP_Totem_C"))
      (Variables|Default|SetMaxNumbersofTotam (Utilities|Array|Length _outactors))
      (EventDispatchers|AssignAllActiveTotam (delegate Custom|AllActiveTotam_Event_0)))
    (:then_6
      ;[1 1 1] PlayerIsDead
      (EventDispatchers|AssignPlayerDead (Variables|Default|GetPlayer%20Refer) (delegate Custom|PlayerDead)))
    (:then_7
      ;[1 1 1] Get Number Of Enemy Bosses , If in the Boss Level
      (bind _returnvalue_4 (Game|GetCurrentLevelName true))
      (if (Utilities|Enum|Equal(Enum) _returnvalue_4 "BossLevel")
        (bind _outactors_2 (Actor|GetAllActorsOfClass "/Game/HeroCharacter/Enemy/BP_EnemyBoss.BP_EnemyBoss_C"))
        (Variables|Default|SetNumber%20of%20Enemy%20Boss%20at%20Level (Utilities|Array|Length _outactors_2))))))

(fn ConstructionScript)

(fn HideHeroCharacter
  (bind _player_refer (Variables|Default|GetPlayer%20Refer))
  (Rendering|SetActorHiddenInGame _player_refer true)
  (Rendering|SetActorHiddenInGame (Variables|/Game/HeroCharacter/BP_Player.BP_Player_C|GetSKGun_Refer _player_refer) false))

(fn UnHideHeroCharacter0
  (bind _player_refer (Variables|Default|GetPlayer%20Refer))
  (Rendering|SetActorHiddenInGame _player_refer false)
  (Rendering|SetActorHiddenInGame (Variables|/Game/HeroCharacter/BP_Player.BP_Player_C|GetSKGun_Refer _player_refer) false))

(fn PossessCheckPoint
  (bind _outactors (Actor|GetAllActorsOfClass "/Game/HeroCharacter/Object/CheckPoint/BP_CheckPoint.BP_CheckPoint_C"))
  (Pawn|Possess (Game|GetPlayerController 0) (Utilities|Array|Get(acopy) _outactors)))

(fn StopAllEnemies
  (bind _outactors (Actor|GetAllActorsOfClass "/Game/HeroCharacter/Enemy/Enemy_BP.Enemy_BP_C"))
  (for _array_element _outactors
    (Default|StopEnemy _array_element)))

(fn AddDeadMenuHidePlayerHUD
  (bind _returnvalue (Game|GetPlayerController 0))
  (bind _menu_dead (Variables|Default|GetMenu%20Dead))
  (Widget|RemovefromParent (Variables|Default|GetHUDPlayerRefer))
  (UserInterface|Viewport|AddtoViewport _menu_dead 0)
  (Input|SetInputModeUIOnly _returnvalue _menu_dead "DoNotLock")
  (Variables|/Script/Engine.PlayerController|SetbShowMouseCursor _returnvalue true))

(fn PossesPlayer
  (Pawn|Possess (Game|GetPlayerController 0) (Variables|Default|GetPlayer%20Refer)))

(fn SetPlayerPosition
  (bind _player_refer (Variables|Default|GetPlayer%20Refer))
  (bind _outactors (Actor|GetAllActorsOfClass "/Game/HeroCharacter/Object/CheckPoint/BP_CheckPoint.BP_CheckPoint_C"))
  (Transformation|SetActorTransform _player_refer (Transformation|GetActorTransform (Utilities|Array|Get(acopy) _outactors)))
  (Pawn|SetControlRotation (Pawn|GetController _player_refer) (Transformation|GetActorRotation (Utilities|Array|Get(acopy) _outactors))))

(fn RemoveDeadMenuHidePlayerHUD0
  (bind _returnvalue (Game|GetPlayerController 0))
  (Widget|RemovefromParent (Variables|Default|GetMenu%20Dead))
  (UserInterface|Viewport|AddtoViewport (Variables|Default|GetHUDPlayerRefer) 0)
  (Input|SetInputModeGameOnly _returnvalue)
  (Variables|/Script/Engine.PlayerController|SetbShowMouseCursor _returnvalue true))

(fn RestartPlayer
  (bind _player_refer (Variables|Default|GetPlayer%20Refer))
  (Variables|/Game/HeroCharacter/BP_Player.BP_Player_C|SetCurrentHealth _player_refer 1e+02)
  (Variables|/Game/HeroCharacter/BP_Player.BP_Player_C|SetIsDead _player_refer false)
  (Default|PlayerResetDeadState _player_refer))

(fn RestartAllEnemies
  (bind _outactors (Actor|GetAllActorsOfClass "/Game/HeroCharacter/Enemy/Enemy_BP.Enemy_BP_C"))
  (for _array_element _outactors
    (Default|RestartEnemyFire _array_element)
    (Default|RestartEnemy _array_element)))

(fn IncreamentNumberKeys
  (bind _result (Math|Integer|IncrementInt (Variables|Default|GetNumberKeysPickup))
    (:%20%20
      (if (== _result 3)
        (Development|PrintString "I Got All Keys")))))

(fn CheckAllActiveTotam
  (if (== (Variables|Default|GetNumberOfTotam) (Variables|Default|GetMaxNumbersofTotam))
    (Default|CallAllActiveTotam)))

(fn IncreamentNumberTotamActive
  (Math|Integer|IncrementInt (Variables|Default|GetNumberOfTotam)))

(fn CheckifNumberEnemyBossEqualDead
  (return (== (Variables|Default|GetNumber%20of%20Enemy%20Boss%20at%20Level) (Variables|Default|GetNumber%20Of%20Enemy%20Bosses%20Dead))))

(fn CheckWin
  (bind _allenemybossdead (CallFunction|CheckifNumberEnemyBossEqualDead))
  (if _allenemybossdead
    (Game|SpawnActorfromClass "/Game/HeroCharacter/Portal/BP_PortalFrame.BP_PortalFrame_C" (Variables|Default|GetPortalLevelSpawnTransform) "Undefined" 0 "Level03" 0)))